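; BP_ShootIt_Character is the first-person character for ShootIt, handling an interact-dot UI and cannon firing.
; Each Tick, a 500-unit camera line trace toggles the dot widget, created on BeginPlay, when it hits an InteractInterface actor.
; Separately, capsule overlap stores a cannon reference, never cleared on exit, and E fires that cannon if it has not yet fired.
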(event `self.ReceiveBeginPlay`
  ;[0 0 0] Loads & Sets Variable for "Interact Dot" UI
  (bind _returnvalue (`|CreateWidget` "/Game/BP_UI_Widgets/InteractDot/InteractDotWidget.InteractDotWidget_C"))
  (set `self.InteractDotWidget` _returnvalue))

(event `self.ReceiveTick`
  (params (DeltaSeconds :type "Float (single-precision)"))
  (bind _interactdotwidget (`self.InteractDotWidget`))
  (bind _returnvalue (`Widget.IsInViewport` (`self.InteractDotWidget`)))
  ;[0 0 0] Checks for interactive actor with Line Trace and adds to viewport when necessary
  (`self.InteractDotWidget`
    (:`then`
      (bind (_returnvalue_2 _outhit) (`self.InteractWidgetLineTrace`))
      (if _returnvalue_2
        (if (`KismetSystemLibrary.DoesImplementInterface` (`.HitActor` (`GameplayStatics.BreakHitResult` _outhit)) "/Game/BP_UI_Widgets/InteractDot/InteractInterface.InteractInterface_C")
          (if (not _returnvalue)
            (`UserWidget.AddToViewport` _interactdotwidget 0))
          (else
            (if _returnvalue :!label _label
              (`Widget.RemoveFromParent` _interactdotwidget))))
        (else
          (goto _label))))
    (:`else`)))

(event `self.CapsuleComponent.OnComponentBeginOverlap`
  (params (OverlappedComponent :type "PrimitiveComponent Object Reference") (OtherActor :type "Actor Object Reference") (OtherComp :type "PrimitiveComponent Object Reference") (OtherBodyIndex :type Integer) (bFromSweep :type Boolean) (SweepResult :type "HitResult Structure (by ref)"))
  (bind _asbp_shoot_it_cannon (cast `/Game/Blueprints/ShootIt/BP_ShootIt_Cannon` OtherActor))
  (set `self.Cannon` _asbp_shoot_it_cannon))

(event `Key|E`
  (params (Key :type "Key Structure"))
  (:`Pressed`
    (bind _cannon (`self.Cannon`)
      (:`then`
        (if (not (`/Game/Blueprints/ShootIt/BP_ShootIt_Cannon.HasFired?` _cannon))
          (`/Game/Blueprints/ShootIt/BP_ShootIt_Cannon.Fire` _cannon)))
      (:`else`))))

(event `Key|Q`
  (params (Key :type "Key Structure")))

(fn `InteractWidgetLineTrace`
  (returns (ReturnValue :type Boolean) (OutHit :type "HitResult Structure"))
  (bind _firstpersoncameracomponent (`self.FirstPersonCameraComponent`))
  (bind _returnvalue (`SceneComponent.K2_GetComponentLocation` _firstpersoncameracomponent))
  (bind (_outhit _returnvalue_2) (`KismetSystemLibrary.LineTraceSingle` _returnvalue (+ _returnvalue (* (`SceneComponent.GetForwardVector` _firstpersoncameracomponent) 500.0)) "TraceTypeQuery1"))
  (return _returnvalue_2 _outhit))

(fn `UserConstructionScript`
  (`parent.UserConstructionScript`))