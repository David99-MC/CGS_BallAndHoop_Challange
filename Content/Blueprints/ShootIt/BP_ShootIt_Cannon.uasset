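; BP_ShootIt_Cannon is a cannon actor for ShootIt that launches a first-person template projectile.
; Its Fire function spawns the projectile at the FirePoint component's location, with a scaled muzzle particle effect and a firing sound.
; HasFired resets on BeginPlay and is set by Fire, but nothing here reads it.
; The event graph's only Fire call is unconnected, so this Blueprint never fires by itself.
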(event `self.ReceiveBeginPlay`
  (set `self.HasFired?` false))

(fn `Fire`
  (`|SpawnActorFromClass` "/Game/FirstPerson/Blueprints/BP_FirstPersonProjectile.BP_FirstPersonProjectile_C" (`KismetMathLibrary.MakeTransform` (`SceneComponent.K2_GetComponentLocation` (`self.FirePoint`))) "AdjustIfPossibleButDontSpawnIfColliding" "MultiplyWithRoot" self null)
  (`GameplayStatics.SpawnEmitterAtLocation` "/Game/GabrielAguiarProd/ToonProjectilesVol1/Particles/Muzzles/P_Muzzle_MegaBomb01Blue.P_Muzzle_MegaBomb01Blue" (`SceneComponent.K2_GetComponentLocation` (`self.FirePoint`)) (struct) (* (`self.MuzzleBaseSize`) (`self.MuzzleScale`)))
  (`GameplayStatics.PlaySoundAtLocation` "/Game/FPWeapon/Audio/FirstPersonTemplateWeaponFire02.FirstPersonTemplateWeaponFire02" (`SceneComponent.K2_GetComponentLocation` (`self.FirePoint`)) (struct) 1.0 1.0 0.0 null null null null)
  (set `self.HasFired?` true))

(fn `UserConstructionScript`)