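; Player character for JustAddWater that uses a held SquirtGun, which either shoots water or acts as a basketball to release.
; Each tick it tilts the GripPoint by the negated pitch difference between control and actor rotation, keeping a fixed yaw offset.
; On left click, a basketball is detached in world space and flagged as released, while any other valid SquirtGun calls ShootWater.
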(event `self.ReceiveBeginPlay`)

(event `self.ReceiveTick`
  (params (DeltaSeconds :type "Float (single-precision)"))
  (`self.Set Grip Point Rotation`))

(event `Key|LeftMouseButton`
  (params (Key :type "Key Structure"))
  (:`Pressed`
    (bind _squirt_gun (`self.Squirt Gun`)
      (:`then`
        (if (`/Game/Blueprints/JustAddWater/BP_SquirtGun.IsBasketBall?` _squirt_gun)
          (`self.K2_DetachFromActor` _squirt_gun "KeepWorld" "KeepWorld" "KeepWorld")
          (set `/Game/Blueprints/JustAddWater/BP_SquirtGun.HasReleased?` true _squirt_gun)
          (else
            (`/Game/Blueprints/JustAddWater/BP_SquirtGun.Shoot Water` _squirt_gun))))
      (:`else`))))

(fn `Set Grip Point Rotation`
  (bind (_returnvalue_roll _returnvalue_pitch) (`KismetMathLibrary.BreakRotator` (`KismetMathLibrary.NormalizedDeltaRotator` (`Controller.GetControlRotation` (`GameplayStatics.GetPlayerController` 0)) (`self.K2_GetActorRotation`))))
  (`SceneComponent.K2_SetRelativeRotation` (`self.Grip Point`) (`KismetMathLibrary.MakeRotator` (* _returnvalue_pitch -1.0) 0.0 -95.0) false false))

(fn `UserConstructionScript`)