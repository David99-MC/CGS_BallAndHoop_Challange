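; Squirt gun pickup for the JustAddWater character that can switch into a basketball.
; On overlap it registers with the character, attaches to the grip point and shows an aiming reticule, with the muzzle following camera rotation each tick.
; ShootWater spawns a projectile and muzzle effect unless in basketball mode.
; SwitchActiveObject swaps visible meshes, StartSimulatePhysics enables ball physics, and once released Tick lerps the actor toward a target location.
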(event `self.ReceiveBeginPlay`
  (set `self.IsBasketBall?` false)
  (set `self.HasReleased?` false)
  ;[0 0 0] Adds retiucle for aiming the squirt gun
  (bind _returnvalue (`|CreateWidget` "/Game/BP_UI_Widgets/InteractDot/InteractDotWidget.InteractDotWidget_C"))
  (set `self.AimingReticule` _returnvalue))

(event `self.ReceiveActorBeginOverlap`
  (params (OtherActor :type "Actor Object Reference"))
  (bind _asbp_just_add_water_character (cast `/Game/Blueprints/JustAddWater/BP_JustAddWater_Character` OtherActor))
  (bind _output_get (set `self.Just Add Water Character` _asbp_just_add_water_character))
  (set `/Game/Blueprints/JustAddWater/BP_JustAddWater_Character.Squirt Gun` self _output_get)
  (bind _returnvalue (`self.K2_AttachToComponent` self (`/Game/Blueprints/JustAddWater/BP_JustAddWater_Character.Grip Point` _asbp_just_add_water_character) "None" "SnapToTarget" "SnapToTarget" "SnapToTarget" true))
  (set `self.IsEquipped?` _returnvalue) ; Variable for the level blueprint\nto call for removing level text
  (`UserWidget.AddToViewport` (`self.AimingReticule`) 0))

(event `self.ReceiveTick`
  (params (DeltaSeconds :type "Float (single-precision)"))
  (bind _just_add_water_character (`self.Just Add Water Character`)
    (:`then`
      (bind _returnvalue (`self.Get Player Camera Rotation` _just_add_water_character))
      (if (`self.HasReleased?`)
        (`self.Set Ball Location` DeltaSeconds)
        (else
          (`SceneComponent.K2_SetWorldRotation` (`self.Muzzle Point`) _returnvalue false false))))
    (:`else`)))

(event `Start Simulate Physics`
  (`PrimitiveComponent.SetCollisionEnabled` (`self.Collision`) "NoCollision")
  (`PrimitiveComponent.SetSimulatePhysics` (`self.Basket Ball`) true)
  (`SceneComponent.K2_DetachFromComponent` (`self.Squirt Gun`) "KeepWorld" "KeepWorld" "KeepWorld" true))

(fn `Get Player Camera Rotation`
  (params (self2 :type "Pawn Object Reference"))
  (returns (ReturnValue :type "Rotator Structure"))
  (return (`PlayerCameraManager.GetCameraRotation` (`PlayerController.PlayerCameraManager` (`Pawn.GetLocalViewingPlayerController` self2)))))

(fn `Set Ball Location`
  (params (Alpha :type "Float (single-precision)"))
  (`self.K2_SetActorLocation` (`KismetMathLibrary.VLerp` (`self.K2_GetActorLocation`) (`self.TargetLocation`) Alpha)))

(fn `Shoot Water`
  (bind _muzzle_point (`self.Muzzle Point`))
  (bind _returnvalue (`SceneComponent.K2_GetComponentLocation` _muzzle_point))
  (if (not (`self.IsBasketBall?`))
    (`|SpawnActorFromClass` "/Game/Blueprints/JustAddWater/BP_WaterProjectile.BP_WaterProjectile_C" (`KismetMathLibrary.MakeTransform` _returnvalue (`SceneComponent.K2_GetComponentRotation` _muzzle_point) (0.4 0.4 0.4)) "AdjustIfPossibleButDontSpawnIfColliding" "MultiplyWithRoot" self null)
    (`GameplayStatics.SpawnEmitterAtLocation` "/Game/GabrielAguiarProd/ToonProjectilesVol1/Particles/Muzzles/P_Muzzle_Waterball01Blue.P_Muzzle_Waterball01Blue" _returnvalue (struct) (0.5 0.5 0.5))))

(fn `Switch Active Object`
  (set `self.IsBasketBall?` true)
  (`SceneComponent.SetVisibility` (`self.Basket Ball`) true false)
  (`SceneComponent.SetVisibility` (`self.Squirt Gun`) false false))

(fn `UserConstructionScript`)