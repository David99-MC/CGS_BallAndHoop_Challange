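; BP_WaterProjectile is the water shot in the JustAddWater game that grows a basketball hoop on hit.
; On overlap it spawns a splash particle, then, for hoop actors only, enlarges the Hoop component by a fixed step and destroys itself.
; When the hoop's scale nears a target size, the owning BP_SquirtGun switches to basketball mode, showing the ball and hiding the gun.
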(event `self.ReceiveActorBeginOverlap`
  (params (OtherActor :type "Actor Object Reference"))
  (`GameplayStatics.SpawnEmitterAtLocation` "/Game/GabrielAguiarProd/ToonProjectilesVol1/Particles/Hits/P_Hit_Waterball01Blue.P_Hit_Waterball01Blue" (`self.K2_GetActorLocation` OtherActor))
  (bind _asbp_just_add_water_hoop (cast `/Game/Blueprints/JustAddWater/BP_JustAddWater_Hoop` OtherActor))
  (bind _hoop (`/Game/Blueprints/JustAddWater/BP_JustAddWater_Hoop.Hoop` _asbp_just_add_water_hoop))
  (`SceneComponent.SetWorldScale3D` _hoop (+ (`SceneComponent.K2_GetComponentScale` _hoop) (0.2 0.2 0.2)))
  (if (== (`SceneComponent.K2_GetComponentScale` (`/Game/Blueprints/JustAddWater/BP_JustAddWater_Hoop.Hoop` _asbp_just_add_water_hoop)) (1.2 1.2 1.2) :`ErrorTolerance` 0.2)
    (bind _asbp_squirt_gun (cast `/Game/Blueprints/JustAddWater/BP_SquirtGun` (`self.GetOwner`)))
    (set `/Game/Blueprints/JustAddWater/BP_SquirtGun.IsBasketBall?` true _asbp_squirt_gun)
    (`SceneComponent.SetVisibility` (`/Game/Blueprints/JustAddWater/BP_SquirtGun.Basket Ball` _asbp_squirt_gun) true false)
    (`SceneComponent.SetVisibility` (`/Game/Blueprints/JustAddWater/BP_SquirtGun.Squirt Gun` _asbp_squirt_gun) false false))
  (`self.K2_DestroyActor`))

(fn `UserConstructionScript`)