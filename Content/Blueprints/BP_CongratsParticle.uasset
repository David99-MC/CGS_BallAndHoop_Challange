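; BP_CongratsParticle is a win trigger actor that ends the game when the player's BP_SquirtGun overlaps it.
; On BeginPlay it creates and stores the WidBP_YouWin widget.
; On overlap it spawns a scaled-up hit particle at its Sphere, plays a crowd cheer, shows the widget, then quits the game after a short delay.
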(event `self.ReceiveBeginPlay`
  ;[0 0 0] Loads and saves "You WIn" widget as variable
  (bind _returnvalue (`|CreateWidget` "/Game/BP_UI_Widgets/WidBP_YouWin.WidBP_YouWin_C"))
  (set `self.YouWInUI` _returnvalue))

(event `self.ReceiveActorBeginOverlap`
  (params (OtherActor :type "Actor Object Reference"))
  (cast `/Game/Blueprints/JustAddWater/BP_SquirtGun` OtherActor)
  (`GameplayStatics.SpawnEmitterAtLocation` "/Game/FXVarietyPack/Particles/P_ky_hit2.P_ky_hit2" (`SceneComponent.K2_GetComponentLocation` (`self.Sphere`)) (struct) (3.0 3.0 3.0))
  (`GameplayStatics.PlaySound2D` "/Game/Blueprints/ShootIt/crowd-yay.crowd-yay" 1.0 1.0 0.0 null null)
  ;[0 0 0] Shows "You Win" widget before automatically closing game
  (`UserWidget.AddToViewport` (`self.YouWinUI`) 0)
  (`KismetSystemLibrary.Delay` 3.0)
  (`KismetSystemLibrary.QuitGame` null "Quit"))

(fn `UserConstructionScript`)