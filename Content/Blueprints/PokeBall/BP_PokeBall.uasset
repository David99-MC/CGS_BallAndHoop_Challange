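; BP_PokeBall is a Pokeball pickup that attaches to the player character's grip point on overlap and flags itself as equipped for the level blueprint.
; Once released, Tick lerps it toward a target location.
; SpawnLazer fires a lightning effect and sound, reveals the basketball hoop after a short delay, then turns on ball physics.
; ComebackToPlayer is an empty stub.
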(event `self.ReceiveActorBeginOverlap`
  (params (OtherActor :type "Actor Object Reference"))
  (bind _asbp_poke_ball_character (cast `/Game/Blueprints/PokeBall/BP_PokeBall_Character` OtherActor))
  (set `self.Poke Ball Character` _asbp_poke_ball_character)
  (set `/Game/Blueprints/PokeBall/BP_PokeBall_Character.Basket Ball` self _asbp_poke_ball_character)
  (bind _returnvalue (`self.K2_AttachToComponent` (`/Game/Blueprints/PokeBall/BP_PokeBall_Character.Grip Point` _asbp_poke_ball_character) "None" "SnapToTarget" "SnapToTarget" "SnapToTarget"))
  (set `self.Has Released?` false)
  (set `self.IsEquipped?` _returnvalue) ; Variable for the level blueprint\nto call from cast
)

(event `self.ReceiveTick`
  (params (DeltaSeconds :type "Float (single-precision)"))
  (if (`self.Has Released?`)
    (`self.K2_SetActorLocation` (`KismetMathLibrary.VLerp` (`self.K2_GetActorLocation`) (`self.Target Location`) (* DeltaSeconds (`self.Move Speed`))))))

(event `SpawnLazer`
  (`GameplayStatics.SpawnEmitterAtLocation` "/Game/FXVarietyPack/Particles/P_ky_lightning3.P_ky_lightning3" (`SceneComponent.K2_GetComponentLocation` (`self.Laser Location`)) (struct) (3.0 3.0 3.0))
  (`GameplayStatics.PlaySound2D` "/Game/Blueprints/PokeBall/poke_sound.poke_sound" 1.0 1.0 0.0 null null)
  (bind _returnvalue (`GameplayStatics.GetActorOfClass` "/Game/Blueprints/ShootIt/BP_ShootIt_BasketballHoop.BP_ShootIt_BasketballHoop_C"))
  (`KismetSystemLibrary.Delay` 0.35)
  (`SceneComponent.SetVisibility` (`StaticMeshActor.StaticMeshComponent` _returnvalue) true false)
  (`KismetSystemLibrary.Delay` 1.0)
  (`PrimitiveComponent.SetSimulatePhysics` (`self.Basket Ball`) true))

(event `Comeback To Player`)

(fn `UserConstructionScript`)